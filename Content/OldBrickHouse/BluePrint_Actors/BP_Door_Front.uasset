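; BP_Door_Front is a front door that the player opens and closes through an Interact event when the character holds the door key.
; BeginPlay caches the player as a PhasmophobiaCharacter, whose HasDoorKey flag gates both directions.
; A FlipFlop alternates between playing the Open timeline with a 2D sound and reversing it silently, with the timeline driving the door mesh's yaw.
; The FlipFlop precedes the key check, so keyless interactions still toggle it.
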(event Custom|MoveDoor
  (bind _openodor (Timeline|Open Reverse)
    (:Update
      (Transformation|SetRelativeRotation (Variables|Default|GetSM_Door_Front) (Math|Rotator|MakeRotator 0.0 0.0 _openodor) false false))))

(event Custom|OpenDoorSound
  (Audio|PlaySound2D "/Game/Audio/open_door_Cue.open_door_Cue" 1.0 1.0 0.0 0 0))

(event Custom|OpenDoor
  (bind _openodor (Timeline|Open Play)
    (:Update
      (Transformation|SetRelativeRotation (Variables|Default|GetSM_Door_Front) (Math|Rotator|MakeRotator 0.0 0.0 _openodor) false false))))

(event EventInteract
  (bind _char_ref (Variables|Default|GetChar%20REF))
  (bind _hasdoorkey (Variables|/Game/Character/PhasmophobiaCharacter.PhasmophobiaCharacter_C|GetHasDoorKey _char_ref))
  (Utilities|FlowControl|FlipFlop
    (:A
      (if _hasdoorkey
        (CallFunction|OpenDoorSound)
        (CallFunction|OpenDoor)))
    (:B
      (if _hasdoorkey
        (CallFunction|MoveDoor)))))

(event EventBeginPlay
  (bind _asphasmophobia_character (Utilities|Casting|CastToPhasmophobiaCharacter (Game|GetPlayerCharacter 0)))
  (Variables|Default|SetChar%20REF _asphasmophobia_character))

(fn ConstructionScript)