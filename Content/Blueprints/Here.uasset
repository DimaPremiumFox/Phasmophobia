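; Trigger-zone actor that opens a menu when a BP_PhasmophobiaCharacter steps into its Box, gated on Steam availability.
; On overlap it checks for the Steam online subsystem, then either shows the Menu widget with the mouse cursor or a YouNotHaveSteam notice that removes itself after a short delay.
; Leaving the box hides the cursor and removes whichever widget is valid.
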(event OnComponentBeginOverlap(Box)
  (params (OverlappedComponent :type Primitive%20Component%20Object%20Reference) (OtherActor :type Actor%20Object%20Reference) (OtherComp :type Primitive%20Component%20Object%20Reference) (OtherBodyIndex :type Integer) (bFromSweep :type Boolean) (SweepResult :type Hit%20Result%20Structure%20%28by%20ref%29))
  (Utilities|Casting|CastToBP_PhasmophobiaCharacter OtherActor)
  (if (Class|AdvancedSessionsLibrary|HasOnlineSubsystem "STEAM")
    (bind _returnvalue (UserInterface|CreateWidget "/Game/Widgets/Menu.Menu_C"))
    (bind _output_get (Variables|Default|SetMenu _returnvalue))
    (UserInterface|Viewport|AddtoViewport _output_get 0)
    (Variables|/Script/Engine.PlayerController|SetbShowMouseCursor (Game|GetPlayerController 0) true)
    (else
      (bind _returnvalue_2 (UserInterface|CreateWidget "/Game/Widgets/YouNotHaveSteam.YouNotHaveSteam_C"))
      (bind _output_get_2 (Variables|Default|SetNoSteam _returnvalue_2))
      (UserInterface|Viewport|AddtoViewport _output_get_2 0)
      (Utilities|FlowControl|Delay 5.0)
      (Widget|RemovefromParent _output_get_2))))

(event OnComponentEndOverlap(Box)
  (params (OverlappedComponent :type Primitive%20Component%20Object%20Reference) (OtherActor :type Actor%20Object%20Reference) (OtherComp :type Primitive%20Component%20Object%20Reference) (OtherBodyIndex :type Integer))
  (Utilities|Casting|CastToBP_PhasmophobiaCharacter OtherActor)
  (Variables|/Script/Engine.PlayerController|SetbShowMouseCursor (Game|GetPlayerController 0) false)
  (bind _menu (Variables|Default|GetMenu)
    (:then
      (Widget|RemovefromParent _menu))
    (:else
      _))
  (bind _nosteam (Variables|Default|GetNoSteam)
    (:then
      (Widget|RemovefromParent _nosteam))
    (:else)))

(event EventBeginPlay)

(event Collision|EventActorBeginOverlap
  (params (OtherActor :type Actor%20Object%20Reference)))

(event EventTick
  (params (DeltaSeconds :type Float%20%28single-precision%29)))

(fn ConstructionScript)